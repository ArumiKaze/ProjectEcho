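; BP_Turret is an enemy turret Blueprint built to fire BP_Projectile actors.
; A timeline update spawns a projectile at SpawnProjectilePosition and pushes its sphere along the Arrow's forward vector with a mass-independent force.
; A Canshoot flag and a one-second delay throttle the fire rate.
; Nothing in the graph starts the timeline, so the firing logic is marked as never running.
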(fn ConstructionScript)